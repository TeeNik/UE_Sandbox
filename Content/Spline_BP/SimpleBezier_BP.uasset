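; Quadratic Bezier actor, apparently a work in progress, that defines a curve from its location through a control anchor to an end point.
; BeginPlay converts both relative points to world space.
; Helpers evaluate position by nested lerps and rotation by finite differences; CreateSpline adds spline meshes, setting only start positions.
; The timeline movement with debug lines is disconnected, and nothing here calls CreateSpline or the unfinished DrawCurve.
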(event EventBeginPlay
  (Variables|Default|SetStart (Transformation|GetActorLocation))
  (CallFunction|UpdatetoWorldVector (Variables|Default|GetControlAnchor))
  (CallFunction|UpdatetoWorldVector (Variables|Default|GetEnd)))

(fn ConstructionScript)

(fn GetLocationBezier
  (params (Start :type Vector) (Anchor :type Vector) (End :type Vector) (Time :type Float%20%28double-precision%29))
  (Utilities|FlowControl|Sequence
    (:then_0
      (LocalVariables|SetTempA (Math|Vector|Lerp(Vector) Start Anchor Time))
      (LocalVariables|SetTempB (Math|Vector|Lerp(Vector) Anchor End Time)))
    (:then_1
      (return (Math|Vector|Lerp(Vector) (LocalVariables|GetTempA) (LocalVariables|GetTempB) Time)))))

(fn GetRotationBezier
  (params (Start :type Vector) (Anchor :type Vector) (End :type Vector) (Time :type Float%20%28double-precision%29))
  (bind _returnvalue (- Time 0.001))
  (LocalVariables|SetTempCurrent (CallFunction|GetLocationBezier Start Anchor End Time))
  (if (Math|Float|InRange(Float) _returnvalue 0.0 1.0)
    (return (Math|Conversions|RotationFromXVector (Math|Vector|Normalize (- (LocalVariables|GetTempCurrent) (CallFunction|GetLocationBezier Start Anchor End _returnvalue)))))
    (else
      (return (Math|Conversions|RotationFromXVector (Math|Vector|Normalize (- (CallFunction|GetLocationBezier Start Anchor End (+ Time 0.001)) (LocalVariables|GetTempCurrent))))))))

(fn UpdatetoWorldVector
  (params (InVector :type Vector%20%28by%20ref%29))
  (|SetBy-RefVar InVector (Math|Transform|TransformLocation (Transformation|GetActorTransform) InVector)))

(fn DrawCurve
  (LocalVariables|SetTempStart (Transformation|GetActorLocation))
  (Variables|Default|SetControlAnchor (Math|Transform|TransformLocation (Transformation|GetActorTransform) (Variables|Default|GetControlAnchor)))
  (LocalVariables|SetTempEnd (Math|Transform|TransformLocation (Transformation|GetActorTransform) (Variables|Default|GetEnd))))

(fn CreateSpline
  (for _index (range 0 (LocalVariables|GetNumOfPoints))
    (bind _returnvalue (AddComponent|AddSplineMeshComponent false))
    (SplineMesh|SetForwardAxis _returnvalue "X" true)
    (SplineMesh|SetStartPosition _returnvalue (CallFunction|GetLocationBezier (Variables|Default|GetStart) (Variables|Default|GetControlAnchor) (Variables|Default|GetEnd) (/ _index (Math|Conversions|ToFloat(Integer) (LocalVariables|GetNumOfPoints)))) true)))