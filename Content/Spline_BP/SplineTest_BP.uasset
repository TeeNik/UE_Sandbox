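; A test spline actor that builds a chain of deformed meshes along its Spline component.
; The construction script adds one collision-enabled spline mesh per segment, oriented on the X axis and fitted to the neighboring points' local positions and tangents.
; The last segment's end is scaled down, tapering the tip of the chain.
; The event graph holds only empty default events, so it adds no runtime logic.
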(event EventBeginPlay)

(event Collision|EventActorBeginOverlap
  (params (OtherActor :type Actor%20Object%20Reference)))

(event EventTick
  (params (DeltaSeconds :type Float%20%28single-precision%29)))

(fn ConstructionScript
  (bind _spline (Variables|Default|GetSpline))
  (bind _spline_2 (Variables|Default|GetSpline))
  (bind _spline_3 (Variables|Default|GetSpline))
  (bind _returnvalue (Spline|GetNumberOfSplinePoints _spline))
  (bind _returnvalue_2 (- _returnvalue 2))
  (for _index (range 0 _returnvalue_2)
    (bind _returnvalue_3 (AddComponent|AddSplineMeshComponent false))
    (SplineMesh|SetForwardAxis _returnvalue_3 "X" true)
    (Collision|SetCollisionEnabled _returnvalue_3 "QueryAndPhysics")
    (SplineMesh|SetStartandEnd _returnvalue_3 (Spline|GetLocationatSplinePoint _spline_3 _index "Local") (Spline|GetTangentatSplinePoint _spline_3 _index "Local") (Spline|GetLocationatSplinePoint _spline_2 (+ _index 1) "Local") (Spline|GetTangentatSplinePoint _spline_2 (+ _index 1) "Local") true :!class /Script/Engine.SplineMeshComponent)
    (if (== _index _returnvalue_2)
      (SplineMesh|SetEndScale _returnvalue_3 "(X=0.250000,Y=0.250000)" true :!class /Script/Engine.SplineMeshComponent))))